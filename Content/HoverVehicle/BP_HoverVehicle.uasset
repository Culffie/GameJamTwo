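; BP_HoverVehicle is a player-controlled hover vehicle that flies by moving and rotating the actor directly, without physics forces.
; Throttle input eases DesiredSpeed toward full forward or half-speed reverse, and Tick smooths CurrentSpeed toward it as a per-frame local X offset.
; Yaw, pitch and strafe inputs apply local rotations and offsets unscaled by delta time.
; Roll input is bound but applies zero rotation.
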(event EventTick
  (params (DeltaSeconds :type Float%20%28single-precision%29))
  ;[1 1 1] Tick - Move Forward/Backward
  (bind _output_get (Variables|Default|SetCurrentSpeed (Math|Interpolation|FInterpTo (Variables|Default|GetCurrentSpeed) (Variables|Default|GetDesiredSpeed) (Utilities|Time|GetWorldDeltaSeconds) (/ (Variables|Default|GetAccelerationInterp) 2.0))))
  (Transformation|AddActorLocalOffset (Math|Vector|MakeVector _output_get 0.0 0.0) false false))

(event Input|AxisEvents|InputAxisIncreaseThrottle
  (params (AxisValue :type Float%20%28single-precision%29))
  ;[1 1 1] Throttle
  (if (> AxisValue 0.0)
    (Variables|Default|SetDesiredSpeed (Math|Interpolation|FInterpTo (Variables|Default|GetDesiredSpeed) (Variables|Default|GetMaxSpeed) (Utilities|Time|GetWorldDeltaSeconds) (Variables|Default|GetAccelerationInterp)))
    (elif (< AxisValue 0.0)
      (Variables|Default|SetDesiredSpeed (Math|Interpolation|FInterpTo (Variables|Default|GetDesiredSpeed) (* (/ (Variables|Default|GetMaxSpeed) 2.0) -1.0) (Utilities|Time|GetWorldDeltaSeconds) (Variables|Default|GetAccelerationInterp))))))

(event Input|AxisEvents|InputAxisYaw
  (params (AxisValue :type Float%20%28single-precision%29))
  ;[1 1 1] Yaw and Pitch
  (if (!= AxisValue 0.0)
    (Transformation|AddActorLocalRotation (Math|Rotator|MakeRotator 0.0 0.0 AxisValue) false false)))

(event Input|AxisEvents|InputAxisPitch
  (params (AxisValue :type Float%20%28single-precision%29))
  ;[1 1 1] Yaw and Pitch
  (if (!= AxisValue 0.0)
    (Transformation|AddActorLocalRotation (Math|Rotator|MakeRotator 0.0 AxisValue 0.0) false false)))

(event Input|AxisEvents|InputAxisMoveRight
  (params (AxisValue :type Float%20%28single-precision%29))
  ;[1 1 1] Strafing
  (if (!= AxisValue 0.0)
    (Transformation|AddActorLocalOffset (Math|Vector|MakeVector 0.0 (* AxisValue (Variables|Default|GetStrafeSpeed)) 0.0) false false)))

(event Input|AxisEvents|InputAxisMoveUp
  (params (AxisValue :type Float%20%28single-precision%29))
  ;[1 1 1] Strafing
  (if (!= AxisValue 0.0)
    (Transformation|AddActorLocalOffset (Math|Vector|MakeVector 0.0 0.0 (* AxisValue (Variables|Default|GetStrafeSpeed))) false false)))

(event Input|AxisEvents|InputAxisRoll
  (params (AxisValue :type Float%20%28single-precision%29))
  (if (!= AxisValue 0.0)
    (Transformation|AddActorLocalRotation (Math|Rotator|MakeRotator 0.0 0.0 0.0) false false)))

(fn ConstructionScript)