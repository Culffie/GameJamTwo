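; Checkpoint actor that registers when a BP_HoverVehicle passes through it in the correct direction.
; When the vehicle leaves the trigger, a dot product of its velocity with the Arrow's forward vector confirms forward travel.
; A valid pass calls CallCheckpointsPassed with CheckpointCount, then hides the trigger and particle effect and disables overlap events, so the checkpoint counts only once.
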(event OnComponentEndOverlap(CheckpointTrigger)
  (params (OverlappedComponent :type Primitive%20Component%20Object%20Reference) (OtherActor :type Actor%20Object%20Reference) (OtherComp :type Primitive%20Component%20Object%20Reference) (OtherBodyIndex :type Integer))
  (bind _checkpointtrigger (Variables|Default|GetCheckpointTrigger))
  ;[1 1 1] Checkpoint System
  (bind _asbp_hover_vehicle (Utilities|Casting|CastToBP_HoverVehicle OtherActor))
  (if (> (Math|Vector|DotProduct (Transformation|GetVelocity _asbp_hover_vehicle) (Math|Rotator|GetRotationXVector (Transformation|GetWorldRotation (Variables|Default|GetArrow)))) 0.0)
    (Default|CallCheckpointsPassed (Variables|Default|GetCheckpointCount))
    (Development|SetHiddeninGame _checkpointtrigger true false)
    (Variables|/Script/Engine.PrimitiveComponent|SetbGenerateOverlapEvents _checkpointtrigger false)))

(fn ConstructionScript)