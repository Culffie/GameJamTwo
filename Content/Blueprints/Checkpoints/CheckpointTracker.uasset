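; Checkpoint tracker for a lap-based race, set up as a skeleton whose helper functions are still stubs.
; On BeginPlay it caches the first player controller, calls Update, then loops over Checkpoints to count them, activate the first and bind each one's passed callback.
; CheckpointCleared forwards the next checkpoint to CurrentLap.
; Update, CurrentLap and ActivateNextCheckpoint are empty, and RaceCompleteCheck returns false and is never reached.
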(event Custom|ApplySettings
  ;[1 1 1] Apply user settings
  (Variables|LapSettings|SetTotalLaps (Variables|LapSettings|GetTotalLaps))
  (CallFunction|Update))

(event Custom|StartSeq
  (bind _checkpoints (Variables|Checkpoints|GetCheckpoints))
  ;[1 1 1] Start Sequence
  (for (_ _array_index) (Variables|Checkpoints|GetCheckpoints)
    (Variables|Default|SetTotalCheckpoints (+ _array_index 1))
    (Variables|Default|SetTotalCheckpoints (Utilities|Array|Length _checkpoints))
    (CallFunction|ActivateNextCheckpoint (Utilities|Array|Get(acopy) _checkpoints))
    (for _array_element (Variables|Checkpoints|GetCheckpoints)
      (EventDispatchers|AssignCheckpointsPassed _array_element (delegate Custom|Checkpoint%20Cleared)))))

(event Custom|Checkpoint%20Cleared
  (params (NextCheckpoint :type Integer))
  (CallFunction|CurrentLap NextCheckpoint))

(event EventBeginPlay
  (bind _asplayer_controller (Utilities|Casting|CastToPlayerController (Game|GetPlayerController 0)))
  (Variables|Default|SetControllerReference _asplayer_controller)
  (CallFunction|ApplySettings)
  (CallFunction|StartSeq))

(fn ConstructionScript)

(fn Update)

(fn CurrentLap
  (params (Checkpoint :type Integer)))

(fn ActivateNextCheckpoint
  (params (ActivateNextCheckpoint :type Checkpoint%20Object%20Reference)))

(fn RaceCompleteCheck
  (return false))