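; Power-up spawner actor that places a Power_Up_Test at its own transform and spawns another after being overlapped.
; Tick spawns whenever the Spawned flag is false, then sets it, so the first power-up appears once play starts.
; Any actor overlap, with no filter on the other actor, clears the flag after a short delay to trigger the next spawn.
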(event EventBeginPlay
  (Variables|Default|SetSpawned false)
  (Collision|SetCollisionEnabled (Variables|Default|GetBox) "QueryOnly"))

(event Collision|EventActorBeginOverlap
  (params (OtherActor :type Actor%20Object%20Reference))
  (Utilities|FlowControl|Delay 2.0)
  (Variables|Default|SetSpawned false))

(event EventTick
  (params (DeltaSeconds :type Float%20%28single-precision%29))
  (if (not (Variables|Default|GetSpawned))
    (Game|SpawnActorfromClass "/Game/Blueprints/PowerUPs/Power_Up_Test.Power_Up_Test_C" (Transformation|GetActorTransform) "Undefined" 0 0)
    (Variables|Default|SetSpawned true)))

(fn ConstructionScript)