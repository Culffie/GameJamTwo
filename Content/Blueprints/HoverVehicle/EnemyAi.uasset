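; AI hover vehicle that follows a spline track once StartHover enables its Tick.
; A downward sphere trace holds it above and aligned to the surface, or drops and levels it when airborne, shaking the player's camera on landing.
; It yaws toward a look-ahead spline point with a periodically randomized sideways offset, then moves forward with a swept offset.
; Hit temporarily raises its speed.
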(event Custom|Line%20trace%20safety
  (bind _returnvalue (Utilities|Time|GetWorldDeltaSeconds))
  (bind _returnvalue_2 (Math|Rotator|MakeRotator 0.0 0.0 0.0))
  (bind _returnvalue_3 (Transformation|GetActorRotation))
  (bind _cube (Variables|Default|GetCube))
  (bind _returnvalue_4 (Transformation|GetWorldLocation _cube))
  (bind _returnvalue_5 (Math|Interpolation|RInterpTo _returnvalue_3 _returnvalue_2 _returnvalue 6.0))
  ;[1 1 1] Track Hover and Alignment
  (bind (_outhit _returnvalue_6) (Collision|SphereTraceByChannel _returnvalue_4 (+ (* (Math|Vector|GetUpVector _cube) -4e+02) _returnvalue_4) 6e+01 "TraceTypeQuery1" false 0 "ForOneFrame"))
  (if _returnvalue_6
    (Transformation|SetActorRotation (Math|Interpolation|RInterpTo (Transformation|GetActorRotation) (Math|Rotator|MakeRotfromZX (.ImpactNormal (Collision|BreakHitResult _outhit)) (Transformation|GetActorForwardVector)) _returnvalue 6.0))
    (Transformation|SetActorLocation (+ (.ImpactPoint (Collision|BreakHitResult _outhit)) (* (.ImpactNormal (Collision|BreakHitResult _outhit)) 1.5e+02)) false false)
    (Utilities|FlowControl|DoOnce true :!label _label
      (:Completed
        (Class|PlayerController|ClientPlayCameraShake (Game|GetPlayerController 0) 0 0.7 "CameraLocal" "0, 0, 0")))
    (else
      (Transformation|AddActorWorldOffset "0, 0,-60.000000")
      (Transformation|SetActorRotation (Math|Rotator|MakeRotator (.roll _returnvalue_5) (.pitch _returnvalue_5) (.Yaw (Math|Rotator|BreakRotator _returnvalue_3))))
      (goto _label Reset))))

(event EventTick
  (params (DeltaSeconds :type Float%20%28single-precision%29))
  (bind _cube (Variables|Default|GetCube))
  (bind _reaction_distance (Variables|Default|GetReaction%20Distance))
  (bind _splinereference (Variables|Default|GetSplineReference))
  (bind _returnvalue (Transformation|GetWorldLocation _cube))
  (bind _usefulspline (Variables|/Game/Blueprints/HoverVehicle/Track.Track_C|GetUsefulSpline _splinereference))
  (bind _returnvalue_2 (Spline|FindDirectionClosesttoWorldLocation _usefulspline _returnvalue "World"))
  (bind _returnvalue_3 (* _returnvalue_2 _reaction_distance))
  (bind _returnvalue_4 (+ _returnvalue_3 _returnvalue))
  ;[1 1 1] Enemy AI
  (CallFunction|LineTraceSafety)
  (Utilities|FlowControl|Delay DeltaSeconds)
  (Utilities|FlowControl|Sequence
    (:then_0
      (Transformation|SetActorRotation (Math|Transform|TransformRotation (Transformation|GetActorTransform) (Math|Rotator|MakeRotator 0.0 0.0 (Math|Interpolation|FInterpTo (.yaw (Variables|/Script/Engine.SceneComponent|GetRelativeRotation (Variables|Default|GetCube))) (.yaw (Math|Transform|InverseTransformRotation (Transformation|GetActorTransform) (Math|Rotator|FindLookatRotation (Transformation|GetActorLocation) (+ (Spline|FindLocationClosesttoWorldLocation _usefulspline _returnvalue_4 "World") (* (Class|SplineComponent|FindRightVectorClosesttoWorldLocation _usefulspline _returnvalue_4 "World") (* (Variables|Default|GetAi%20Prefered%20Location) 1.0)))))) (Utilities|Time|GetWorldDeltaSeconds) 0.0))))
      (Transformation|AddActorLocalOffset (stale Collision|EventHit _output_get) true false))
    (:then_1
      (Utilities|FlowControl|Delay (Math|Random|RandomFloatinRange 1.0 4.0))
      (Variables|Default|SetAi%20Prefered%20Location (Math|Random|RandomFloatinRange -1e+03 1e+03)))))

(event EventStartHover
  (Actor|Tick|SetActorTickEnabled true))

(event EventBeginPlay
  (Actor|Tick|SetActorTickEnabled false))

(event Collision|EventHit
  (params (MyComp :type Primitive%20Component%20Object%20Reference) (Other :type Actor%20Object%20Reference) (OtherComp :type Primitive%20Component%20Object%20Reference) (bSelfMoved :type Boolean) (HitLocation :type Vector :default "0, 0, 0") (HitNormal :type Vector :default "0, 0, 0") (NormalImpulse :type Vector :default "0, 0, 0") (Hit :type Hit%20Result%20Structure%20%28by%20ref%29))
  ;[1 1 1] Enemy AI
  ;;[1 1 1] Physics for collision
  (bind _output_get (Variables|Default|SetMax%20Speed "250.000000, 0, 0"))
  (Utilities|FlowControl|RetriggerableDelay 3.0)
  (Variables|Default|SetMax%20Speed "200.000000, 0, 0"))

(fn ConstructionScript)

(fn SplitAxis
  (params (Value :type Float%20%28single-precision%29))
  (return (Math|Float|Clamp(Float) Value) (Math|Float|Clamp(Float) (- 0.0 Value))))