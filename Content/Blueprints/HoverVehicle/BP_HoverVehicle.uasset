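; Player-driven hover vehicle that follows track surfaces, with movement idle until the StartHover countdown event enables Tick.
; Throttle eases a desired speed that Tick smooths into swept forward/reverse movement, while yaw input also rolls.
; A downward sphere trace holds hover height and aligns to the surface normal, shaking the camera on contact; without ground it falls and levels out.
; Hits briefly raise max speed; strafe logic is unwired.
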(event Custom|Line%20trace%20safety
  (bind _returnvalue (Utilities|Time|GetWorldDeltaSeconds))
  (bind _returnvalue_2 (Math|Rotator|MakeRotator 0.0 0.0 0.0))
  (bind _returnvalue_3 (Transformation|GetActorRotation))
  (bind _cube (Variables|Default|GetCube))
  (bind _returnvalue_4 (Transformation|GetWorldLocation _cube))
  (bind _returnvalue_5 (Math|Interpolation|RInterpTo _returnvalue_3 _returnvalue_2 _returnvalue 6.0))
  ;[1 1 1] Track Hover and Alignment
  (bind (_outhit _returnvalue_6) (Collision|SphereTraceByChannel _returnvalue_4 (+ (* (Math|Vector|GetUpVector _cube) -4e+02) _returnvalue_4) 6e+01 "TraceTypeQuery1" false 0 "ForOneFrame"))
  (if _returnvalue_6
    (Transformation|SetActorRotation (Math|Interpolation|RInterpTo (Transformation|GetActorRotation) (Math|Rotator|MakeRotfromZX (.ImpactNormal (Collision|BreakHitResult _outhit)) (Transformation|GetActorForwardVector)) _returnvalue 6.0))
    (Transformation|SetActorLocation (+ (.ImpactPoint (Collision|BreakHitResult _outhit)) (* (.ImpactNormal (Collision|BreakHitResult _outhit)) 1.5e+02)) false false)
    (Utilities|FlowControl|DoOnce true :!label _label
      (:Completed
        (Class|PlayerController|ClientPlayCameraShake (Game|GetPlayerController 0) "/Script/Engine.CameraShake" 0.7 "CameraLocal" "0, 0, 0")))
    (else
      (Transformation|AddActorWorldOffset "0, 0,-60.000000")
      (Transformation|SetActorRotation (Math|Rotator|MakeRotator (.roll _returnvalue_5) (.pitch _returnvalue_5) (.Yaw (Math|Rotator|BreakRotator _returnvalue_3))))
      (goto _label Reset))))

(event EventStartHover
  ;[1 1 1] Countdown Interface
  (Actor|Tick|SetActorTickEnabled true))

(event EventBeginPlay
  ;[1 1 1] Countdown Interface
  (Actor|Tick|SetActorTickEnabled false))

(event EventTick
  (params (DeltaSeconds :type Float%20%28single-precision%29))
  ;[1 1 1] Tick - Move Forward/Backward
  (bind _output_get (Variables|Default|SetCurrentSpeed (Math|Interpolation|FInterpTo (Variables|Default|GetCurrentSpeed) (Variables|Default|GetDesiredSpeed) (Utilities|Time|GetWorldDeltaSeconds) (/ (Variables|Default|GetAccelerationInterp) 2.0))))
  (Transformation|AddActorLocalOffset (Math|Vector|MakeVector _output_get 0.0 0.0) true false)
  (CallFunction|LineTraceSafety))

(event Collision|EventHit
  (params (MyComp :type Primitive%20Component%20Object%20Reference) (Other :type Actor%20Object%20Reference) (OtherComp :type Primitive%20Component%20Object%20Reference) (bSelfMoved :type Boolean) (HitLocation :type Vector :default "0, 0, 0") (HitNormal :type Vector :default "0, 0, 0") (NormalImpulse :type Vector :default "0, 0, 0") (Hit :type Hit%20Result%20Structure%20%28by%20ref%29))
  ;[1 1 1] Physics for collision
  (Development|PrintString (Utilities|String|ToString(Float) (stale _output_get)))
  (bind _output_get (Variables|Default|SetMaxSpeed 5e+02))
  (Utilities|FlowControl|RetriggerableDelay 3.0)
  (Development|PrintString (Utilities|String|ToString(Float) (stale _output_get_2)))
  (bind _output_get_2 (Variables|Default|SetMaxSpeed 4e+02)))

(event Input|AxisEvents|InputAxisIncreaseThrottle
  (params (AxisValue :type Float%20%28single-precision%29))
  ;[1 1 1] Throttle
  (if (> AxisValue 0.0)
    (Variables|Default|SetDesiredSpeed (Math|Interpolation|FInterpTo (Variables|Default|GetDesiredSpeed) (Variables|Default|GetMaxSpeed) (Utilities|Time|GetWorldDeltaSeconds) (Variables|Default|GetAccelerationInterp)))
    (elif (< AxisValue 0.0)
      (Variables|Default|SetDesiredSpeed (Math|Interpolation|FInterpTo (Variables|Default|GetDesiredSpeed) (* (/ (Variables|Default|GetMaxSpeed) 2.0) -1.0) (Utilities|Time|GetWorldDeltaSeconds) (Variables|Default|GetAccelerationInterp)))
      (elif (== AxisValue 0.0)
        (Variables|Default|SetDesiredSpeed (Math|Interpolation|FInterpTo (Variables|Default|GetDesiredSpeed) 0.0 (Utilities|Time|GetWorldDeltaSeconds) 0.0))))))

(event Input|AxisEvents|InputAxisYaw
  (params (AxisValue :type Float%20%28single-precision%29))
  ;[1 1 1] Yaw and Pitch
  (if (!= AxisValue 0.0)
    (Transformation|AddActorLocalRotation (Math|Rotator|MakeRotator AxisValue 0.0 AxisValue) false false)))

(fn ConstructionScript)

(fn SplitAxis
  (params (Value :type Float%20%28single-precision%29))
  (return (Math|Float|Clamp(Float) Value) (Math|Float|Clamp(Float) (- 0.0 Value))))